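; BP_FlamePillar is a flame pillar actor that continuously flickers its FireLight.
; On BeginPlay it randomly picks one of two FlameIntensity timelines, and whenever one finishes it picks again, so the flicker varies without a fixed loop.
; Each timeline update feeds ScaleFlameIntensity, which multiplies the curve value by BaseIntensity to set the light's intensity.
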(event Custom|StartTimeline_01
  (bind _flameintensity (Timeline|FlameIntensity_01 PlayFromStart)
    (:Update
      (CallFunction|ScaleFlameIntensity _flameintensity))
    (:Finished
      (CallFunction|ChooseTimeline))))

(event Custom|StartTImeline_02
  (bind _flameintensity (Timeline|FlameIntensity_02 PlayFromStart)
    (:Update
      (CallFunction|ScaleFlameIntensity _flameintensity))
    (:Finished
      (CallFunction|ChooseTimeline))))

(event Custom|ChooseTimeline
  (switch int (Math|Random|RandomIntegerinRange 0 1)
    (:Default
      (CallFunction|StartTImeline02 :!label _label))
    (:0
      (CallFunction|StartTimeline01))
    (:1
      (goto _label))))

(event EventBeginPlay
  (CallFunction|ChooseTimeline))

(event Collision|EventActorBeginOverlap
  (params (OtherActor :type Actor%20Object%20Reference)))

(event EventTick
  (params (DeltaSeconds :type Float%20%28single-precision%29)))

(fn ConstructionScript)

(fn ScaleFlameIntensity
  (params (Intensity :type Float%20%28double-precision%29))
  (Rendering|Components|Light|SetIntensity (Variables|Default|GetFireLight) (* Intensity (Variables|Default|GetBaseIntensity))))